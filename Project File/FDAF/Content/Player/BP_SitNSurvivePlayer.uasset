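; Player pawn for SitNSurvive, a seated player who switches between four fixed views: left, straight, right and behind.
; Each look input records the view index for other Blueprints and triggers a timeline lerp of the camera from its current transform, ignoring repeated inputs.
; VisionBox collision is off during moves; its overlaps notify actors when they are looked at or away from.
; Game over locks camera switching; a separate event enables physics on the camera's collision box.
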(event OnComponentBeginOverlap(VisionBox)
  (params (OverlappedComponent :type Primitive%20Component%20Object%20Reference) (OtherActor :type Actor%20Object%20Reference) (OtherComp :type Primitive%20Component%20Object%20Reference) (OtherBodyIndex :type Integer) (bFromSweep :type Boolean) (SweepResult :type Hit%20Result%20Structure%20%28by%20ref%29))
  (Class|BPIPlayerActionResponse|Lookedat(Message) OtherActor))

(event OnComponentEndOverlap(VisionBox)
  (params (OverlappedComponent :type Primitive%20Component%20Object%20Reference) (OtherActor :type Actor%20Object%20Reference) (OtherComp :type Primitive%20Component%20Object%20Reference) (OtherBodyIndex :type Integer))
  (Class|BPIPlayerActionResponse|NoLongerLookedat(Message) OtherActor))

(event Custom|MoveCamera
  (params (TargetPlayercamLocation :type Vector) (TargetPlayercamRotation :type Rotator) (Can%20Move? :type Boolean))
  (bind _visionbox (Variables|Default|GetVisionBox))
  (bind _visionbox_2 (Variables|Default|GetVisionBox))
  (if Can%20Move?
    (Collision|SetCollisionEnabled _visionbox "NoCollision")
    (Development|SetHiddeninGame _visionbox false false)
    (CallFunction|InitializeCameraMovement TargetPlayercamLocation TargetPlayercamRotation)
    (bind _output (Timeline|TL_ChangePlayerCameraAngle PlayFromStart)
      (:Update
        (CallFunction|LerpComponentLocationandRotation (Variables|Default|GetCamera) _output (Variables|Default|GetPreviousPlayercamLocation) (Variables|Default|GetTargetPlayercamLocation) (Variables|Default|GetPreviousPlayercamRotation) (Variables|Default|GetTargetPlayercamRotation)))
      (:Finished
        (Collision|SetCollisionEnabled _visionbox_2 "QueryOnly")
        (Development|SetHiddeninGame _visionbox_2 false false)))))

(event Input|EnhancedActionEvents|EnhancedInputActionIA_LookLeft
  (params (ActionValue :type Boolean) (ElapsedSeconds :type Float%20%28double-precision%29) (TriggeredSeconds :type Float%20%28double-precision%29) (InputAction :type Input%20Action%20Object%20Reference :default "/Game/Player/Input/IAs/IA_LookLeft.IA_LookLeft"))
  (:Started
    (CallFunction|MoveCamera "340.000000,40.000000,490.000000" "-2.000000,120.000000,-4.000000" (and (!= InputAction (Variables|Default|GetLastInputAction)) (Variables|Default|GetCanMoveCamera?)))
    (Variables|Default|SetPlayerCam 0)
    (Variables|Default|SetLastInputAction InputAction)))

(event Input|EnhancedActionEvents|EnhancedInputActionIA_LookRight
  (params (ActionValue :type Boolean) (ElapsedSeconds :type Float%20%28double-precision%29) (TriggeredSeconds :type Float%20%28double-precision%29) (InputAction :type Input%20Action%20Object%20Reference :default "/Game/Player/Input/IAs/IA_LookRight.IA_LookRight"))
  (:Started
    (CallFunction|MoveCamera "340.000000,40.000000,490.000000" "-2.000000,-120.000000,-4.000000" (and (!= InputAction (Variables|Default|GetLastInputAction)) (Variables|Default|GetCanMoveCamera?)))
    (Variables|Default|SetPlayerCam 2)
    (Variables|Default|SetLastInputAction InputAction)))

(event Input|EnhancedActionEvents|EnhancedInputActionIA_LookStraight
  (params (ActionValue :type Boolean) (ElapsedSeconds :type Float%20%28double-precision%29) (TriggeredSeconds :type Float%20%28double-precision%29) (InputAction :type Input%20Action%20Object%20Reference :default "/Game/Player/Input/IAs/IA_LookStraight.IA_LookStraight"))
  (:Started
    (CallFunction|MoveCamera "502.000000,-17.000000,500.000000" "0.000000,-180.000000,0.000000" (and (!= InputAction (Variables|Default|GetLastInputAction)) (Variables|Default|GetCanMoveCamera?)))
    (Variables|Default|SetPlayerCam 1)
    (Variables|Default|SetLastInputAction InputAction)))

(event Input|EnhancedActionEvents|EnhancedInputActionIA_lookBehind
  (params (ActionValue :type Boolean) (ElapsedSeconds :type Float%20%28double-precision%29) (TriggeredSeconds :type Float%20%28double-precision%29) (InputAction :type Input%20Action%20Object%20Reference :default "/Game/Player/Input/IAs/IA_lookBehind.IA_lookBehind"))
  (:Started
    (CallFunction|MoveCamera "502.000000,-107.000000,553.000000" "0, 0, 0" (and (!= InputAction (Variables|Default|GetLastInputAction)) (Variables|Default|GetCanMoveCamera?)))
    (Variables|Default|SetPlayerCam 3)
    (Variables|Default|SetLastInputAction InputAction)))

(event EventBeginPlay
  ;[0.15 0.15 0.15 0.5] Gives player the SitNSurvive Input Map
  (Input|AddMappingContext (PlayerController|LocalPlayerSubsystems|GetEnhancedInputLocalPlayerSubsystem (Game|GetPlayerController 0)) "/Game/Player/Input/IMC_SitNSurvive.IMC_SitNSurvive" 0 "(bIgnoreAllPressedKeysUntilRelease=True,bForceImmediately=False,bNotifyUserSettings=False)"))

(event EventBeginGameOver
  (Variables|Default|SetCanMoveCamera? false))

(event EventActivateCameraPhysics
  (Physics|SetSimulatePhysics (Variables|Default|GetCameraCollisionBox_0) true))

(event Input|KeyboardEvents|AnyKey
  (params (Key :type Key%20Structure :default "None")))

(fn ConstructionScript)

(fn InitializeCameraMovement
  (params (TargetPlayercamLocation :type Vector) (TargetPlayercamRotation :type Rotator))
  (bind _camera (Variables|Default|GetCamera))
  (Variables|Default|SetPreviousPlayercamLocation (Transformation|GetWorldLocation _camera))
  (Variables|Default|SetPreviousPlayercamRotation (Transformation|GetWorldRotation _camera))
  (Variables|Default|SetTargetPlayercamRotation TargetPlayercamRotation)
  (Variables|Default|SetTargetPlayercamLocation TargetPlayercamLocation))

(fn LerpComponentLocationandRotation
  (params (TargetComponent :type Scene%20Component%20Object%20Reference) (Alpha :type Float%20%28double-precision%29) (PreviousLocation :type Vector) (TargetLocation :type Vector) (PreviousRotation :type Rotator) (TargetRotation :type Rotator))
  (Transformation|SetWorldLocationAndRotation TargetComponent (Math|Vector|Lerp(Vector) (Variables|Default|GetPreviousPlayercamLocation) (Variables|Default|GetTargetPlayercamLocation) Alpha) (Math|Rotator|Lerp(Rotator) (Variables|Default|GetPreviousPlayercamRotation) (Variables|Default|GetTargetPlayercamRotation) Alpha true) false false))

(fn RequestCamLocation
  (return (Variables|Default|GetPlayerCam)))