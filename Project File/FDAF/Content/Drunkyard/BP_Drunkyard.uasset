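; Drunkyard is an enemy that kills the player with a bottle if watched for too long.
; A looping timer teleports it to a random left, middle or right spot, unless it already moved, is on screen or the camera occupies that spot.
; Being looked at starts a kill countdown ending in a timeline-driven bottle flight and game over; looking away in time resets it.
; Higher AI level shortens both timers.
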(event Custom|TryToMove
  (Variables|Default|SetDesiredLocation (Math|Random|RandomInteger 3))
  (bind _output (Class|BPIPlayerInterface|RequestCamLocation(Message) (Game|Player|GetPlayerPawn 0)))
  (if (Math|Boolean|ORBoolean (Variables|Default|GetDrunkyardAlreadyMoved?) (== _output (Variables|Default|GetDesiredLocation)) (CallFunction|CheckifActorIsonScreen))
    (Development|PrintString "move failed")
    (else
      (switch int (Variables|Default|GetDesiredLocation)
        (:Default
          (Development|PrintString "Drunkyard defaulted??"))
        (:0
          (Transformation|SetActorLocationAndRotation "-110.000000,1800.000000,310.000000" "0, 0, 0") ; Left
          (Variables|Default|SetCurrentLocation 0)
          (Variables|Default|SetDrunkyardAlreadyMoved? true)
          (Development|PrintString (Utilities|String|ToString(Text) (Utilities|Text|FormatText "drunkyard moved to {m}" (Variables|Default|GetCurrentLocation))) true true "(R=1.000000,G=0.000000,B=0.879462,A=1.000000)" :!label _label))
        (:1
          (Transformation|SetActorLocationAndRotation "-600.000000,-10.000000,330.000000" "0, 0, 0") ; Middle
          (Variables|Default|SetCurrentLocation 1)
          (Variables|Default|SetDrunkyardAlreadyMoved? true)
          (goto _label))
        (:2
          (Transformation|SetActorLocationAndRotation "-350.000000,-2010.000000,240.000000" "0, 0, 0") ; Right
          (Variables|Default|SetCurrentLocation 2)
          (Variables|Default|SetDrunkyardAlreadyMoved? true)
          (goto _label))))))

(event Custom|Kill%20Player
  (Utilities|FlowControl|DoOnce false
    (:Completed
      (Transformation|SetWorldLocation (Variables|Default|GetBottle) (Transformation|GetWorldLocation (Variables|Default|GetCylinder)) false false)
      (Development|PrintString "DIED" true true "(R=1.000000,G=0.000104,B=0.026893,A=1.000000)" 3.0 "111")
      (Variables|Default|SetKillingPlayer? true)
      (Class|BPIPlayerInterface|BeginGameOver(Message) (Game|Player|GetPlayerPawn 0))
      (bind (_direction _output _vectoradjustment) (Timeline|TL_BottleMovingToCranium Play)
        (:Update
          (Transformation|SetWorldLocation (Variables|Default|GetBottle) (+ _vectoradjustment (Math|Vector|Lerp(Vector) (Transformation|GetWorldLocation (Variables|Default|GetCylinder)) (Transformation|GetWorldLocation (Actor|GetComponentbyClass (Game|Player|GetPlayerPawn 0) "/Script/Engine.CameraComponent")) _output)) false false))
        (:Finished
          (Class|BPIPlayerInterface|ActivateCameraPhysics(Message) (Game|Player|GetPlayerPawn 0)))))))

(event EventBeginPlay
  (Variables|Default|SetMovementTimer (CallFunction|CalculateMovementTime))
  (Variables|Default|SetKillTimer (CallFunction|CalculateKillTime))
  (Development|PrintText (Utilities|Text|FormatText "AI level: {AI} 
MoveTimer: {t} 
KillTimer: {k}" (Variables|Default|GetAI%20Level) (Variables|Default|GetMovementTimer) (Variables|Default|GetKillTimer)) true true "(R=0.000000,G=0.660000,B=1.000000,A=1.000000)" 5e+01)
  (Utilities|Time|SetTimerbyEvent (delegate Custom|TryToMove) (Variables|Default|GetMovementTimer) true))

(event EventLookedat
  (bind _returnvalue (Utilities|Time|SetTimerbyEvent (delegate Custom|Kill%20Player) 0.01 false false (Variables|Default|GetKillTimer)))
  (Variables|Default|SetKillTimerHandle _returnvalue))

(event EventNoLongerLookedat
  (if (not (Variables|Default|GetKillingPlayer?))
    (Utilities|Time|ClearandInvalidateTimerbyHandle (Variables|Default|GetKillTimerHandle))
    (Development|PrintString "aww you got away in time" true true "(R=0.189824,G=1.000000,B=0.000000,A=1.000000)" 3.0 "111")
    (Variables|Default|SetDrunkyardAlreadyMoved? false)
    (Transformation|SetActorLocationAndRotation "0, 0, 0" "0, 0, 0")))

(fn ConstructionScript)

(fn CalculateMovementTime
  (return (- (Math|Float|MakeLiteralFloat 1e+01) (* (Variables|Default|GetAI%20Level) 0.25))))

(fn CalculateKillTime
  (return (- (Math|Float|MakeLiteralFloat 2.5) (* (Variables|Default|GetAI%20Level) 0.1))))

(fn CheckifActorIsonScreen
  (bind _returnvalue (Game|GetPlayerController 0))
  (bind _returnvalue_2 (Viewport|GetViewportSize))
  (bind _returnvalue_3 (Transformation|GetActorLocation))
  (bind _screenlocation (Class|PlayerController|ProjectWorldLocationtoScreen _returnvalue _returnvalue_3 false))
  (return (Math|Boolean|ANDBoolean (> (.x _screenlocation) 0.0) (> (.y _screenlocation) 0.0) (< (.x _screenlocation) (.x _returnvalue_2)) (< (.y _screenlocation) (.y _returnvalue_2)))))